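; BP_FallingSmallRocks is a falling rock hazard or platform that drops when the custom third-person player enters its box trigger, then resets itself.
; An activation delay precedes enabling physics on the rock mesh and playing an attached rock sound.
; After a fall delay, physics turns off and a timeline lerps the rock back to its BeginPlay transform.
; An IsReady flag blocks retriggering until the return finishes.
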(event OnComponentBeginOverlap(BoxTrigger)
  (params (OverlappedComponent :type Primitive%20Component%20Object%20Reference) (OtherActor :type Actor%20Object%20Reference) (OtherComp :type Primitive%20Component%20Object%20Reference) (OtherBodyIndex :type Integer) (bFromSweep :type Boolean) (SweepResult :type Hit%20Result%20Structure%20%28by%20ref%29))
  ;[0.15 0.04035 0.1449 0.5] Falling COde
  ;;[0.15 0.1484 0.1479 0.5] Player Activation
  (Development|PrintString "Somethign ran into my trigger!")
  (if (Variables|Default|GetIsReady)
    (Utilities|Casting|CastToBP_Custom3rdP OtherActor)
    (CallFunction|Activated)))

(event Custom|Activated
  ;[0.15 0.04035 0.1449 0.5] Falling COde
  ;;[0.05924 0.15 0.1232 0.5] Activated Platform
  (Development|PrintString "Activated")
  (Variables|Default|SetIsReady false)
  (Utilities|FlowControl|Delay (Variables|RockSettings|GetActivitaion%20Delay%20Duration))
  (CallFunction|Falling))

(event Custom|Falling
  ;[0.15 0.04035 0.1449 0.5] Falling COde
  ;;[0.15 0.1083 0.02683 0.5] Falling Platform
  (Audio|SpawnSoundAttached "/Game/MyStuff/audio/rock.rock" (Variables|Default|GetSM_RockBigC) "None" "0, 0, 0" "0, 0, 0" "KeepRelativeOffset" false 1.0 1.0 0.0 0 0)
  (Development|PrintString "Falling")
  (Physics|SetSimulatePhysics (Variables|Default|GetSM_RockBigC) true)
  (Utilities|FlowControl|Delay (Variables|RockSettings|GetFall%20Delay%20Duration))
  (CallFunction|Resetting))

(event Custom|Resetting
  ;[0.15 0.04035 0.1449 0.5] Falling COde
  ;;[0.15 0.04112 0.04062 0.5] Resting Platform
  (Development|PrintString "Resetting")
  (Variables|Default|SetFalling%20Transform (Transformation|GetWorldTransform (Variables|Default|GetSM_RockBigC)))
  (Physics|SetSimulatePhysics (Variables|Default|GetSM_RockBigC) false)
  (bind _track (Timeline|returntostart PlayFromStart)
    (:Update
      (Transformation|SetWorldLocationAndRotation (Variables|Default|GetSM_RockBigC) (.location (Math|Transform|Lerp(Transform) (Variables|Default|GetFalling%20Transform) (Variables|Default|GetOriginal%20Transform) _track)) (.rotation (Math|Transform|Lerp(Transform) (Variables|Default|GetFalling%20Transform) (Variables|Default|GetOriginal%20Transform) _track)) false false))
    (:Finished
      (Variables|Default|SetIsReady true))))

(event EventBeginPlay
  ;[0.15 0.04035 0.1449 0.5] Falling COde
  ;;[0.02823 0.1162 0.15 0.5] World Transform
  (Variables|Default|SetOriginal%20Transform (Transformation|GetWorldTransform (Variables|Default|GetSM_RockBigC))))

(fn ConstructionScript)