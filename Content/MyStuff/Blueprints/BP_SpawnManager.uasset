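; BP_SpawnManager handles enemy waves by spawning BP_Enemy actors at the level's BP_SpawnPoint actors.
; Shortly after BeginPlay it runs SpawnEnemies, which loops over every spawn point and gives each a weighted random chance to spawn an enemy.
; NewWaveCheck counts living enemies and, when one or none remains, waits briefly before spawning the next wave.
; Debug prints trace each step.
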(event Custom|Spawn%20Enemies
  ;[0.0736 0.04541 0.15 0.5] Enemy Spawn
  (bind _outactors (Actor|GetAllActorsOfClass "/Game/MyStuff/Blueprints/BP_SpawnPoint.BP_SpawnPoint_C"))
  (for _array_element _outactors
    (Development|PrintString (Utilities|GetDisplayName _array_element) true true "(R=0.490909,G=0.054783,B=1.000000,A=1.000000)" 1e+01)
    (if (Math|Random|RandomBoolwithWeight 0.8)
      (Game|SpawnActorfromClass "/Game/MyStuff/Blueprints/BP_Enemy.BP_Enemy_C" (Transformation|GetWorldTransform (Variables|/Game/MyStuff/Blueprints/BP_SpawnPoint.BP_SpawnPoint_C|GetDefaultSceneRoot _array_element)) "Undefined" "MultiplyWithRoot" 0 0)))
  (Development|PrintString "Finished with the For Each Loop for spawn enemies"))

(event Custom|NewWaveCheck
  ;[0.15 0.08994 0.03982 0.5] New Wave Check
  (Development|PrintString "Was I the last enemy?" true true "(R=0.599037,G=0.180556,B=1.000000,A=1.000000)")
  (bind _outactors (Actor|GetAllActorsOfClass "/Game/MyStuff/Blueprints/BP_Enemy.BP_Enemy_C"))
  (Development|PrintString (Utilities|String|Append " There are " (Utilities|String|ToString(Integer) (Utilities|Array|Length _outactors)) "  enemies") true true "(R=0.141198,G=0.012231,B=0.234375,A=1.000000)")
  (if (> (Utilities|Array|Length _outactors) 1)
    (Development|PrintString "You were not the las one" true true "(R=0.276736,G=0.140878,B=0.427083,A=1.000000)")
    (else
      (Development|PrintString "New Wave In Coming" true true "(R=1.000000,G=0.000000,B=0.000000,A=1.000000)")
      (Utilities|FlowControl|Delay 3.0)
      (CallFunction|SpawnEnemies))))

(event EventBeginPlay
  ;[0.0736 0.04541 0.15 0.5] Enemy Spawn
  (Development|PrintString "Spawn Manager Exist") ; Tell the player we exist
  (Utilities|FlowControl|Delay 1.0)
  (CallFunction|SpawnEnemies))

(fn ConstructionScript)